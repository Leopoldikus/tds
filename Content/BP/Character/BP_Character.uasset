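; Top-down player character Blueprint that turns input into walk, sprint and aim movement states, montages, camera shake and mouse-wheel zoom.
; Input flags feed ChangeMovementState, while Tick uses one-second Delays to drain or regenerate sprint stamina.
; Zoom changes spring arm length instantly or in looping timer steps, and the construction script configures the boom.
; Weapon reload events play montages; cursor-driven aim camera and weapon debug logic are unwired.
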(event `Key|V`
  (params (Key :type "Key Structure"))
  (:`Pressed`
    (`|PlayMontage` (`self.Mesh`) "/Game/BP/Character/Mannequin/Animations/MyNewAnimation/MyDeath_1_Montage.MyDeath_1_Montage")))

(event `Key|SpaceBar`
  (params (Key :type "Key Structure"))
  (bind _mesh (`self.Mesh`))
  (:`Pressed`
    (if (`self.AimEnable`)
      (`|PlayMontage` _mesh "/Game/BP/Character/Mannequin/Animations/MyNewAnimation/MyFire_Rifle_Ironsights_Montage.MyFire_Rifle_Ironsights_Montage")
      (else
        (`|PlayMontage` _mesh "/Game/BP/Character/Mannequin/Animations/MyNewAnimation/MyFire_Rifle_Hip_Montage.MyFire_Rifle_Hip_Montage")))))

(event `Key|F`
  (params (Key :type "Key Structure"))
  (:`Pressed`
    (`self.CameraShakeEvent`)))

(event `InputAxis|MouseWheel`
  (params (AxisValue :type "Float (single-precision)"))
  (if (`self.SlideWithSmooth`)
    (`self.CameraSlideSmooth` AxisValue)
    (else
      (`self.CameraSlide` AxisValue))))

(event `InputAction|MovementModeChangeWalk`
  (params (Key :type "Key Structure"))
  (:`Pressed`
    (set `self.WalkEnable` true)
    (`self.ChangeMovementState` :!label _label))
  (:`Released`
    (set `self.WalkEnable` false)
    (goto _label)))

(event `InputAction|MovementModeChangeSprint`
  (params (Key :type "Key Structure"))
  (:`Pressed`
    (if (>= (`self.Stamina`) 10.0)
      (set `self.SprintRunEnable` true)
      (goto _label)))
  (:`Released`
    (set `self.SprintRunEnable` false)
    (goto _label)))

(event `Key|RightMouseButton`
  (params (Key :type "Key Structure"))
  (:`Pressed`
    (set `self.AimEnable` true)
    (goto _label))
  (:`Released`
    (set `self.AimEnable` false)
    (goto _label)))

(event `self.ReceiveTick`
  (params (DeltaSeconds :type "Float (single-precision)"))
  ;[1 1 1] Stamina increase decrease
  (if (`self.SprintRunEnable`)
    (`KismetSystemLibrary.Delay` 1.0)
    (if (<= (`self.Stamina`) 0.0)
      (set `self.SprintRunEnable` false)
      (`self.ChangeMovementState`)
      (elif (or (!= (.x (`CharacterMovementComponent.GetCurrentAcceleration` (`self.CharacterMovement`))) 0.0) (!= (.y (`CharacterMovementComponent.GetCurrentAcceleration` (`self.CharacterMovement`))) 0.0) (!= (.z (`CharacterMovementComponent.GetCurrentAcceleration` (`self.CharacterMovement`))) 0.0))
        (set `self.Stamina` (- (`self.Stamina`) 10.0))
        (`KismetSystemLibrary.PrintString` (`KismetStringLibrary.Conv_DoubleToString` (`self.Stamina`)) :!label _label_2)))
    (else
      (`KismetSystemLibrary.Delay` 1.0)
      (if (< (`self.Stamina`) (`self.MaxStamina`))
        (set `self.Stamina` (`KismetMathLibrary.FMin` (+ (`self.Stamina`) 15.0) (`self.MaxStamina`)))
        (goto _label_2)))))

(event `self.WeaponReloadStart_BP`
  (params (Anim :type "AnimMontage Object Reference"))
  (`self.PlayAnimMontage` Anim))

(event `self.WeaponReloadEnd_BP`)

(fn `CameraShakeEvent`
  (`GameplayStatics.PlayWorldCameraShake` "/Game/BP/Game/BP_CameraShake.BP_CameraShake_C" (`SceneComponent.K2_GetComponentLocation` (`self.TopDownCameraComponent`)) 0.0 30.0))

(fn `CameraSlide`
  (params (Value :type "Float (double-precision)"))
  (bind _cameraboom (`self.CameraBoom`))
  (bind _heightcamerachangedistance (`self.HeightCameraChangeDistance`))
  (bind _targetarmlength (`SpringArmComponent.TargetArmLength` _cameraboom))
  (bind _returnvalue (- _targetarmlength _heightcamerachangedistance))
  (bind _returnvalue_2 (+ _targetarmlength _heightcamerachangedistance))
  (if (!= Value 0.0)
    (if (< Value 0.0)
      (if (> (`self.CameraHeightMax`) _returnvalue_2)
        (set `SpringArmComponent.TargetArmLength` _returnvalue_2 _cameraboom))
      (elif (< (`self.CameraHeightMin`) _returnvalue)
        (set `SpringArmComponent.TargetArmLength` _returnvalue _cameraboom)))))

(fn `CameraSlideSmooth`
  (params (Value :type "Float (double-precision)"))
  (bind _heightcamerachangedistance (`self.HeightCameraChangeDistance`))
  (bind _targetarmlength (`SpringArmComponent.TargetArmLength` (`self.CameraBoom`)))
  (if (`self.SlideDone`)
    (if (!= Value 0.0)
      (if (< Value 0.0)
        (if (>= (`self.CameraHeightMax`) (+ _targetarmlength _heightcamerachangedistance))
          (set `self.SlideUp` true)
          (set `self.SlideDone` false :!label _label)
          (bind _returnvalue (`KismetSystemLibrary.K2_SetTimer` null "CameraSlideSmoothTick" (`self.TimerStep`) true))
          (set `self.SlideTimer` _returnvalue))
        (elif (<= (`self.CameraHeightMin`) (- _targetarmlength _heightcamerachangedistance))
          (set `self.SlideUp` false)
          (goto _label))))))

(fn `CameraSlideSmoothTick`
  (params (Value :type "Float (double-precision)"))
  (bind _heightcamerachangeslidestepdistance (`self.HeightCameraChangeSlideStepDistance`))
  (bind _cameraboom (`self.CameraBoom`))
  (bind _targetarmlength (`SpringArmComponent.TargetArmLength` _cameraboom))
  (bind _output_get (set `self.CurrentSlideDistance` (+ (`self.CurrentSlideDistance`) _heightcamerachangeslidestepdistance)))
  (set `SpringArmComponent.TargetArmLength` (select `bool` (`self.SlideUp`) :`false` (- _targetarmlength _heightcamerachangeslidestepdistance) :`true` (+ _targetarmlength _heightcamerachangeslidestepdistance)) _cameraboom)
  (if (>= _output_get (`self.HeightCameraChangeDistance`))
    (set `self.CurrentSlideDistance` 0.0)
    (set `self.SlideDone` true)
    (`KismetSystemLibrary.K2_ClearAndInvalidateTimerHandle` (`self.SlideTimer`))))

(fn `SprintDirectionCheck`
  (returns (ReturnValue :type Boolean))
  (return (<= (`KismetMathLibrary.DegAcos` (`KismetMathLibrary.Dot_VectorVector` (`SceneComponent.GetForwardVector` (`self.Mesh`)) (`KismetMathLibrary.Normal` (`self.GetVelocity`)))) 15.0)))

(fn `UserConstructionScript`
  (bind _cameraboom (`self.CameraBoom`))
  (set `SpringArmComponent.TargetArmLength` (`self.Height`) _cameraboom)
  (`SceneComponent.K2_SetRelativeRotation` _cameraboom (`self.Camera Rotator`) false false)
  (set `SpringArmComponent.bEnableCameraLag` (`self.Flow`) _cameraboom)
  (set `SpringArmComponent.CameraLagSpeed` (`self.Smooth_Coef`) _cameraboom))